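; Character class selection Blueprint that shows the Select_Class_WDG widget with a category dropdown defaulting to "Guerrero".
; On BeginPlay and selection changes, it reads the chosen Base_Categoria row and feeds grouped functions for base, combat, mystic, psychic, secondary skill and bonus stats.
; These fill widget texts, mostly through SetTextWitchColor, which colors values by exact match against per-stat tiers and leaves unmatched texts untouched.
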(event Custom|OnSelectionChanged_Event_0
  (params (SelectedItem :type String) (SelectionType :type ESelectInfo%20Enum :default "OnKeyPress"))
  (EventDispatchers|AssignOnSelectionChanged (Variables|/Game/Widgets/Select_Class_WDG.Select_Class_WDG_C|GetDropDown_CategoriaSelect (stale EventBeginPlay _returnvalue)) (delegate Custom|OnSelectionChanged_Event_0))
  (bind _returnvalue (Utilities|GetDataTableRow "/Game/Data/Base_Categoria.Base_Categoria" (Utilities|String|StringToName (Class|ComboBoxString|GetSelectedOption (Variables|/Game/Widgets/Select_Class_WDG.Select_Class_WDG_C|GetDropDown_CategoriaSelect (stale EventBeginPlay _returnvalue)))))
    (:then
      (Utilities|FlowControl|Sequence
        (:then_0
          (|Stats_Base _returnvalue))
        (:then_1
          (|Stats_Combate _returnvalue))
        (:then_2
          (|Stats_Mistico _returnvalue))
        (:then_3
          (|Stats_Psiquicas _returnvalue))
        (:then_4
          (|Stats_Campos_Secundarias _returnvalue))
        (:then_5
          (|OtrosBonos _returnvalue))))))

(event EventBeginPlay
  (Utilities|FlowControl|Delay 0.2)
  (bind _returnvalue (UserInterface|CreateWidget "/Game/Widgets/Select_Class_WDG.Select_Class_WDG_C"))
  (Variables|Default|SetCategorias_WDG _returnvalue)
  (UserInterface|Viewport|AddtoViewport _returnvalue 0)
  (Variables|/Script/Engine.PlayerController|SetbShowMouseCursor (Game|GetPlayerController 0) true)
  (for _array_element (Variables|Default|GetNombres)
    (Class|ComboBoxString|AddOption (Variables|/Game/Widgets/Select_Class_WDG.Select_Class_WDG_C|GetDropDown_CategoriaSelect _returnvalue) (Utilities|String|ToString(Name) _array_element))
    (Class|ComboBoxString|SetSelectedOption (Variables|/Game/Widgets/Select_Class_WDG.Select_Class_WDG_C|GetDropDown_CategoriaSelect _returnvalue) "Guerrero")
    (EventDispatchers|AssignOnSelectionChanged (Variables|/Game/Widgets/Select_Class_WDG.Select_Class_WDG_C|GetDropDown_CategoriaSelect _returnvalue) (delegate Custom|OnSelectionChanged_Event_0))
    (bind _returnvalue_2 (Utilities|GetDataTableRow "/Game/Data/Base_Categoria.Base_Categoria" (Utilities|String|StringToName (Class|ComboBoxString|GetSelectedOption (Variables|/Game/Widgets/Select_Class_WDG.Select_Class_WDG_C|GetDropDown_CategoriaSelect _returnvalue))))
      (:then
        (Utilities|FlowControl|Sequence
          (:then_0
            (|Stats_Base _returnvalue_2))
          (:then_1
            (|Stats_Combate _returnvalue_2))
          (:then_2
            (|Stats_Mistico _returnvalue_2))
          (:then_3
            (|Stats_Psiquicas _returnvalue_2))
          (:then_4
            (|Stats_Campos_Secundarias _returnvalue_2))
          (:then_5
            (|OtrosBonos _returnvalue_2))))))
  (Class|ComboBoxString|RefreshOptions (Variables|/Game/Widgets/Select_Class_WDG.Select_Class_WDG_C|GetDropDown_CategoriaSelect _returnvalue))
  (bind _returnvalue_3 (Utilities|GetDataTableRow "/Game/Data/Base_Categoria.Base_Categoria" (Utilities|String|StringToName (Class|ComboBoxString|GetSelectedOption (Variables|/Game/Widgets/Select_Class_WDG.Select_Class_WDG_C|GetDropDown_CategoriaSelect _returnvalue))))
    (:then
      (Utilities|FlowControl|Sequence
        (:then_0
          (|Stats_Base _returnvalue_3))
        (:then_1
          (|Stats_Combate _returnvalue_3))
        (:then_2
          (|Stats_Mistico _returnvalue_3))
        (:then_3
          (|Stats_Psiquicas _returnvalue_3))
        (:then_4
          (|Stats_Campos_Secundarias _returnvalue_3))
        (:then_5
          (|OtrosBonos _returnvalue_3))))))

(event Collision|EventActorBeginOverlap
  (params (OtherActor :type Actor%20Object%20Reference)))

(event EventTick
  (params (DeltaSeconds :type Float%20%28single-precision%29)))

(fn ConstructionScript)

(fn SetTextWitchColor
  (params (Coste :type Integer) (Rojo :type Integer) (Amarillo :type Integer) (Verde :type Integer) (Azul :type Integer) (Dorado :type Integer) (Blanco :type Integer) (Texto :type Text%20Block%20Object%20Reference))
  (if (== Coste Rojo)
    (LocalVariables|SetColor%20Actual (Utilities|Struct|MakeSlateColor "(R=0.200000,G=0.000000,B=0.000000,A=1.000000)"))
    (Appearance|SetColorandOpacity Texto (stale _output_get) :!class /Script/UMG.TextBlock :!label _label)
    (Rendering|Components|TextRender|SetText Texto (Utilities|Text|ToText(Integer) Coste))
    (elif (== Coste Amarillo)
      (LocalVariables|SetColor%20Actual (Utilities|Struct|MakeSlateColor "(R=0.400000,G=0.100000,B=0.000000,A=1.000000)"))
      (goto _label)
      (elif (== Coste Verde)
        (bind _output_get (LocalVariables|SetColor%20Actual (Utilities|Struct|MakeSlateColor "(R=0.000000,G=0.100000,B=0.000000,A=1.000000)")))
        (goto _label)
        (elif (== Coste Azul)
          (LocalVariables|SetColor%20Actual (Utilities|Struct|MakeSlateColor "(R=0.000000,G=0.050000,B=0.100000,A=1.000000)"))
          (goto _label)
          (elif (== Coste Dorado)
            (LocalVariables|SetColor%20Actual (Utilities|Struct|MakeSlateColor "(R=1.000000,G=0.793067,B=0.115994,A=1.000000)"))
            (goto _label)
            (elif (== Coste Blanco)
              (LocalVariables|SetColor%20Actual (Utilities|Struct|MakeSlateColor "(R=0.708008,G=0.755208,B=0.754879,A=1.000000)"))
              (goto _label))))))))