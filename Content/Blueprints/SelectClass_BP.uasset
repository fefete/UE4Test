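; SelectClass_BP drives a class-selection screen for an Anima character creator, showing each category's archetypes, costs and bonuses.
; Its dropdown handler reads the Base_Categoria data table and passes the row to per-section functions.
; SetTextWitchColor colour-codes numbers by matching per-stat tier values, leaving unmatched fields untouched.
; Widget creation and dropdown setup are disconnected from BeginPlay, alongside an uncoloured SetFields path using GameMode's array.
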(event Custom|CustomEvent
  (params (SelectedItem :type String) (SelectionType :type ESelectInfo%20Enum :default "OnKeyPress"))
  (for _array_element (Variables|/Game/Blueprints/BP_AnimaCreatorGameMode.BP_AnimaCreatorGameMode_C|GetCategoriaArray (Variables|Default|GetGameMode))
    (if (Utilities|Enum|Equal(Enum) SelectedItem (Utilities|String|ToString(Name) (.Categoria (Utilities|Struct|BreakStruct_Categoria _array_element))))
      (CallFunction|SetFields _array_element (Variables|Default|GetCategorias_WDG)))))

(event Custom|OnSelectionChanged_Event_0
  (params (SelectedItem :type String) (SelectionType :type ESelectInfo%20Enum :default "OnKeyPress"))
  (bind _categorias_wdg (Variables|Default|GetCategorias_WDG))
  (bind _dropdown_categoriaselect (Variables|/Game/Widgets/Select_Class_WDG.Select_Class_WDG_C|GetDropDown_CategoriaSelect _categorias_wdg))
  (EventDispatchers|AssignOnSelectionChanged _dropdown_categoriaselect (delegate Custom|OnSelectionChanged_Event_0))
  (bind _returnvalue (Utilities|GetDataTableRow "/Game/Data/Base_Categoria.Base_Categoria" (Utilities|String|StringToName (Class|ComboBoxString|GetSelectedOption _dropdown_categoriaselect)))
    (:then
      (Utilities|FlowControl|Sequence
        (:then_0
          (|Stats_Base _returnvalue))
        (:then_1
          (|Stats_Combate _returnvalue))
        (:then_2
          (|Stats_Mistico _returnvalue))
        (:then_3
          (|Stats_Psiquicas _returnvalue))
        (:then_4
          (|Stats_Campos_Secundarias _returnvalue))
        (:then_5
          (|OtrosBonos _returnvalue))))))

(event EventBeginPlay)

(event Collision|EventActorBeginOverlap
  (params (OtherActor :type Actor%20Object%20Reference)))

(event EventTick
  (params (DeltaSeconds :type Float%20%28single-precision%29)))

(fn ConstructionScript)

(fn SetTextWitchColor
  (params (Coste :type Integer) (Rojo :type Integer) (Amarillo :type Integer) (Verde :type Integer) (Azul :type Integer) (Dorado :type Integer) (Blanco :type Integer) (Texto :type Text%20Block%20Object%20Reference))
  (if (== Coste Rojo)
    (LocalVariables|SetColor%20Actual (Utilities|Struct|MakeSlateColor "(R=0.200000,G=0.000000,B=0.000000,A=1.000000)"))
    (Appearance|SetColorandOpacity Texto (stale _output_get) :!class /Script/UMG.TextBlock :!label _label)
    (Rendering|Components|TextRender|SetText Texto (Utilities|Text|ToText(Integer) Coste))
    (elif (== Coste Amarillo)
      (LocalVariables|SetColor%20Actual (Utilities|Struct|MakeSlateColor "(R=0.400000,G=0.100000,B=0.000000,A=1.000000)"))
      (goto _label)
      (elif (== Coste Verde)
        (bind _output_get (LocalVariables|SetColor%20Actual (Utilities|Struct|MakeSlateColor "(R=0.000000,G=0.100000,B=0.000000,A=1.000000)")))
        (goto _label)
        (elif (== Coste Azul)
          (LocalVariables|SetColor%20Actual (Utilities|Struct|MakeSlateColor "(R=0.000000,G=0.050000,B=0.100000,A=1.000000)"))
          (goto _label)
          (elif (== Coste Dorado)
            (LocalVariables|SetColor%20Actual (Utilities|Struct|MakeSlateColor "(R=1.000000,G=0.793067,B=0.115994,A=1.000000)"))
            (goto _label)
            (elif (== Coste Blanco)
              (LocalVariables|SetColor%20Actual (Utilities|Struct|MakeSlateColor "(R=0.708008,G=0.755208,B=0.754879,A=1.000000)"))
              (goto _label))))))))

(fn SetFields
  (params (Struct :type Struct%20Categoria%20Structure) (Widget :type Select%20Class%20WDG%20Object%20Reference))
  (bind (_categoria _arquetipo _arquetiposecundario _c_pv _b_lvl_pv _b_lvl_turno _b_lvl_cm _b_lvl_cv _limitecombate _c_ataque _c_parada _c_esquiva _c_armadura _c_ki _c_kiacu _limitesobrenatural _c_zeon _c_act _c_projmag _c_convocar _c_dominar _c_atar _c_desconvocar _limite_psi _c_cv _c_projpsi _c_atleticas _c_sociales _c_perceptivas _c_intelectuales _c_vigor _c_subterfugio _c_creativas _b_lvl_ataque _b_lvl_esquiva _b_lvl_parada _b_lvl_armadura _b_zeon _b_convocar _b_dominar _b_atar _b_desconvocar) (Utilities|Struct|BreakStruct_Categoria Struct))
  (CallFunction|SetValueString (Variables|/Game/Widgets/Select_Class_WDG.Select_Class_WDG_C|GetArquetipo Widget) (Utilities|String|ToString(Name) _arquetipo))
  (CallFunction|SetValueString (Variables|/Game/Widgets/Select_Class_WDG.Select_Class_WDG_C|GetArquetipoSecundario Widget) (Utilities|String|ToString(Name) _arquetiposecundario))
  (CallFunction|SetValueInteger (Variables|/Game/Widgets/Select_Class_WDG.Select_Class_WDG_C|GetCostePV Widget) _c_pv)
  (CallFunction|SetValueInteger (Variables|/Game/Widgets/Select_Class_WDG.Select_Class_WDG_C|GetPVxLVL Widget) _b_lvl_pv)
  (CallFunction|SetValueInteger (Variables|/Game/Widgets/Select_Class_WDG.Select_Class_WDG_C|GetTurnoxLvl Widget) _b_lvl_turno)
  (CallFunction|SetValueInteger (Variables|/Game/Widgets/Select_Class_WDG.Select_Class_WDG_C|GetCVxLvl Widget) _b_lvl_cv)
  (CallFunction|SetValueInteger (Variables|/Game/Widgets/Select_Class_WDG.Select_Class_WDG_C|GetCMxLvl Widget) _b_lvl_cm)
  (CallFunction|SetValueInteger (Variables|/Game/Widgets/Select_Class_WDG.Select_Class_WDG_C|GetC_Ataque Widget) _c_ataque)
  (CallFunction|SetValueInteger (Variables|/Game/Widgets/Select_Class_WDG.Select_Class_WDG_C|GetCombate_Limite Widget) _limitecombate)
  (CallFunction|SetValueInteger (Variables|/Game/Widgets/Select_Class_WDG.Select_Class_WDG_C|GetC_Esquiva Widget) _c_esquiva)
  (CallFunction|SetValueInteger (Variables|/Game/Widgets/Select_Class_WDG.Select_Class_WDG_C|GetC_Parada Widget) _c_parada)
  (CallFunction|SetValueInteger (Variables|/Game/Widgets/Select_Class_WDG.Select_Class_WDG_C|GetC_Ki Widget) _c_ki)
  (CallFunction|SetValueInteger (Variables|/Game/Widgets/Select_Class_WDG.Select_Class_WDG_C|GetC_Armadura Widget) _c_armadura)
  (CallFunction|SetValueInteger (Variables|/Game/Widgets/Select_Class_WDG.Select_Class_WDG_C|GetC_Limite_Místico Widget) _limitesobrenatural)
  (CallFunction|SetValueInteger (Variables|/Game/Widgets/Select_Class_WDG.Select_Class_WDG_C|GetC_ACKI Widget) _c_kiacu)
  (CallFunction|SetValueInteger (Variables|/Game/Widgets/Select_Class_WDG.Select_Class_WDG_C|GetC_Zeon Widget) _c_zeon)
  (CallFunction|SetValueInteger (Variables|/Game/Widgets/Select_Class_WDG.Select_Class_WDG_C|GetC_ACT Widget) _c_act)
  (CallFunction|SetValueInteger (Variables|/Game/Widgets/Select_Class_WDG.Select_Class_WDG_C|GetC_ProjM Widget) _c_projmag)
  (CallFunction|SetValueInteger (Variables|/Game/Widgets/Select_Class_WDG.Select_Class_WDG_C|GetC_Conv Widget) _c_convocar)
  (CallFunction|SetValueInteger (Variables|/Game/Widgets/Select_Class_WDG.Select_Class_WDG_C|GetC_Domin Widget) _c_dominar)
  (CallFunction|SetValueInteger (Variables|/Game/Widgets/Select_Class_WDG.Select_Class_WDG_C|GetC_Atar Widget) _c_atar)
  (CallFunction|SetValueInteger (Variables|/Game/Widgets/Select_Class_WDG.Select_Class_WDG_C|GetC_Desconv Widget) _c_desconvocar)
  (CallFunction|SetValueInteger (Variables|/Game/Widgets/Select_Class_WDG.Select_Class_WDG_C|GetC_Limite_Psi Widget) _limite_psi)
  (CallFunction|SetValueInteger (Variables|/Game/Widgets/Select_Class_WDG.Select_Class_WDG_C|GetC_CV Widget) _c_cv)
  (CallFunction|SetValueInteger (Variables|/Game/Widgets/Select_Class_WDG.Select_Class_WDG_C|GetC_Proj_Psi Widget) _c_projpsi)
  (CallFunction|SetValueInteger (Variables|/Game/Widgets/Select_Class_WDG.Select_Class_WDG_C|GetC_Atleticas Widget) _c_atleticas)
  (CallFunction|SetValueInteger (Variables|/Game/Widgets/Select_Class_WDG.Select_Class_WDG_C|GetC_Sociales Widget) _c_sociales)
  (CallFunction|SetValueInteger (Variables|/Game/Widgets/Select_Class_WDG.Select_Class_WDG_C|GetC_Perceptivas Widget) _c_perceptivas)
  (CallFunction|SetValueInteger (Variables|/Game/Widgets/Select_Class_WDG.Select_Class_WDG_C|GetC_Intelectuales Widget) _c_intelectuales)
  (CallFunction|SetValueInteger (Variables|/Game/Widgets/Select_Class_WDG.Select_Class_WDG_C|GetC_Vigor Widget) _c_vigor)
  (CallFunction|SetValueInteger (Variables|/Game/Widgets/Select_Class_WDG.Select_Class_WDG_C|GetC_Subterfugio Widget) _c_subterfugio)
  (CallFunction|SetValueInteger (Variables|/Game/Widgets/Select_Class_WDG.Select_Class_WDG_C|GetC_Creativas Widget) _c_creativas)
  (CallFunction|SetValueInteger (Variables|/Game/Widgets/Select_Class_WDG.Select_Class_WDG_C|GetB_Ataque Widget) _b_lvl_ataque)
  (CallFunction|SetValueInteger (Variables|/Game/Widgets/Select_Class_WDG.Select_Class_WDG_C|GetB_Esquiva Widget) _b_lvl_esquiva)
  (CallFunction|SetValueInteger (Variables|/Game/Widgets/Select_Class_WDG.Select_Class_WDG_C|GetB_Parada Widget) _b_lvl_parada)
  (CallFunction|SetValueInteger (Variables|/Game/Widgets/Select_Class_WDG.Select_Class_WDG_C|GetB_Armadura Widget) _b_lvl_armadura)
  (CallFunction|SetValueInteger (Variables|/Game/Widgets/Select_Class_WDG.Select_Class_WDG_C|GetB_Zeon Widget) _b_zeon)
  (CallFunction|SetValueInteger (Variables|/Game/Widgets/Select_Class_WDG.Select_Class_WDG_C|GetB_Convocar Widget) _b_convocar)
  (CallFunction|SetValueInteger (Variables|/Game/Widgets/Select_Class_WDG.Select_Class_WDG_C|GetB_Dominar Widget) _b_dominar)
  (CallFunction|SetValueInteger (Variables|/Game/Widgets/Select_Class_WDG.Select_Class_WDG_C|GetB_Atar Widget) _b_atar)
  (CallFunction|SetValueInteger (Variables|/Game/Widgets/Select_Class_WDG.Select_Class_WDG_C|GetB_Desconvocar Widget) _b_desconvocar)
  (return))

(fn SetValueString
  (params (Name :type Text%20Block%20Object%20Reference) (Value :type String))
  (Rendering|Components|TextRender|SetText Name (Utilities|Text|ToText(String) Value))
  (return))

(fn SetValueInteger
  (params (Name :type Text%20Block%20Object%20Reference) (Value :type Integer))
  (Rendering|Components|TextRender|SetText Name (Utilities|Text|ToText(Integer) Value))
  (return))