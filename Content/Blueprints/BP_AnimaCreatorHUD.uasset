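; HUD Blueprint for an Anima character creator that shows the class-selection widget with a mouse cursor.
; It fills a category dropdown from the GameMode's CategoriaArray; selecting one copies that struct's costs, limits and per-level bonuses into text fields.
; Macros bind the dropdown and level-box events, with level commits recalculating total PD linearly.
; Characteristic boxes are bound on BeginPlay, but their AttributeChanged handler is an empty switch on object name.
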(event Custom|onCaracteristicaActualChanged
  (params (Text :type Text%20%28by%20ref%29) (CommitMethod :type ETextCommit%20Enum :default "Default"))
  (CallFunction|AttributeChanged (stale EventBeginPlay _astext_box) Text))

(event EventBeginPlay
  (Utilities|FlowControl|Delay 0.2)
  (bind _returnvalue (UserInterface|CreateWidget "/Game/Widgets/Select_Class_WDG.Select_Class_WDG_C" (Game|GetPlayerController 0)))
  (bind _output_get (Variables|Default|SetCategorias_WDG _returnvalue))
  (UserInterface|Viewport|AddtoViewport _output_get 0)
  (Variables|/Script/Engine.PlayerController|SetbShowMouseCursor (Game|GetPlayerController 0) true)
  (bind _asbp_anima_creator_game_mode (Utilities|Casting|CastToBP_AnimaCreatorGameMode (Game|GetGameMode)))
  (bind _output_get_2 (Variables|Default|SetGameMode _asbp_anima_creator_game_mode))
  (for _array_element (Variables|/Game/Blueprints/BP_AnimaCreatorGameMode.BP_AnimaCreatorGameMode_C|GetCategoriaArray _output_get_2)
    (Class|ComboBoxString|AddOption (Variables|/Game/Widgets/Select_Class_WDG.Select_Class_WDG_C|GetDropDown_CategoriaSelect (Variables|Default|GetCategorias_WDG)) (Utilities|String|ToString(Name) (.Categoria (Utilities|Struct|BreakStruct_Categoria _array_element))))
    (Development|PrintString (Utilities|String|ToString(Name) (.Categoria (Utilities|Struct|BreakStruct_Categoria _array_element)))))
  (Utilities|FlowControl|Sequence
    (:then_0
      (|OnChangeLevel (Variables|/Game/Widgets/Select_Class_WDG.Select_Class_WDG_C|GetDropDown_CategoriaSelect (Variables|Default|GetCategorias_WDG))))
    (:then_1
      (|OnLevelChange (Variables|Default|GetCategorias_WDG) (Variables|Default|GetCategorias_WDG)))
    (:then_2
      (for _index (range 0 (Class|PanelWidget|GetChildrenCount (Variables|/Game/Widgets/Select_Class_WDG.Select_Class_WDG_C|GetCaracteristicas_Actual (Variables|Default|GetCategorias_WDG))))
        (bind _astext_box (Utilities|Casting|CastToEditableTextBox (Class|PanelWidget|GetChildat (Variables|/Game/Widgets/Select_Class_WDG.Select_Class_WDG_C|GetCaracteristicas_Actual (Variables|Default|GetCategorias_WDG)) _index)))
        (EventDispatchers|BindEventtoOnTextCommitted _astext_box (delegate Custom|onCaracteristicaActualChanged))))))

(event Collision|EventActorBeginOverlap
  (params (OtherActor :type Actor%20Object%20Reference)))

(event EventTick
  (params (DeltaSeconds :type Float%20%28single-precision%29)))

(fn ConstructionScript)

(fn SetFields
  (params (Struct :type Struct%20Categoria%20Structure) (Widget :type Select%20Class%20WDG%20Object%20Reference))
  (bind (_categoria _arquetipo _arquetiposecundario _c_pv _b_lvl_pv _b_lvl_turno _b_lvl_cm _b_lvl_cv _limitecombate _c_ataque _c_parada _c_esquiva _c_armadura _c_ki _c_kiacu _limitesobrenatural _c_zeon _c_act _c_projmag _c_convocar _c_dominar _c_atar _c_desconvocar _limite_psi _c_cv _c_projpsi _c_atleticas _c_sociales _c_perceptivas _c_intelectuales _c_vigor _c_subterfugio _c_creativas _b_lvl_ataque _b_lvl_esquiva _b_lvl_parada _b_lvl_armadura _b_zeon _b_convocar _b_dominar _b_atar _b_desconvocar) (Utilities|Struct|BreakStruct_Categoria Struct))
  (CallFunction|SetValueString (Variables|/Game/Widgets/Select_Class_WDG.Select_Class_WDG_C|GetArquetipo Widget) (Utilities|String|ToString(Name) _arquetipo))
  (CallFunction|SetValueString (Variables|/Game/Widgets/Select_Class_WDG.Select_Class_WDG_C|GetArquetipoSecundario Widget) (Utilities|String|ToString(Name) _arquetiposecundario))
  (CallFunction|SetValueInteger (Variables|/Game/Widgets/Select_Class_WDG.Select_Class_WDG_C|GetCostePV Widget) _c_pv)
  (CallFunction|SetValueInteger (Variables|/Game/Widgets/Select_Class_WDG.Select_Class_WDG_C|GetPVxLVL Widget) _b_lvl_pv)
  (CallFunction|SetValueInteger (Variables|/Game/Widgets/Select_Class_WDG.Select_Class_WDG_C|GetTurnoxLvl Widget) _b_lvl_turno)
  (CallFunction|SetValueInteger (Variables|/Game/Widgets/Select_Class_WDG.Select_Class_WDG_C|GetCVxLvl Widget) _b_lvl_cv)
  (CallFunction|SetValueInteger (Variables|/Game/Widgets/Select_Class_WDG.Select_Class_WDG_C|GetCMxLvl Widget) _b_lvl_cm)
  (CallFunction|SetValueInteger (Variables|/Game/Widgets/Select_Class_WDG.Select_Class_WDG_C|GetC_Ataque Widget) _c_ataque)
  (CallFunction|SetValueInteger (Variables|/Game/Widgets/Select_Class_WDG.Select_Class_WDG_C|GetCombate_Limite Widget) _limitecombate)
  (CallFunction|SetValueInteger (Variables|/Game/Widgets/Select_Class_WDG.Select_Class_WDG_C|GetC_Esquiva Widget) _c_esquiva)
  (CallFunction|SetValueInteger (Variables|/Game/Widgets/Select_Class_WDG.Select_Class_WDG_C|GetC_Parada Widget) _c_parada)
  (CallFunction|SetValueInteger (Variables|/Game/Widgets/Select_Class_WDG.Select_Class_WDG_C|GetC_Ki Widget) _c_ki)
  (CallFunction|SetValueInteger (Variables|/Game/Widgets/Select_Class_WDG.Select_Class_WDG_C|GetC_Armadura Widget) _c_armadura)
  (CallFunction|SetValueInteger (Variables|/Game/Widgets/Select_Class_WDG.Select_Class_WDG_C|GetC_Limite_Místico Widget) _limitesobrenatural)
  (CallFunction|SetValueInteger (Variables|/Game/Widgets/Select_Class_WDG.Select_Class_WDG_C|GetC_ACKI Widget) _c_kiacu)
  (CallFunction|SetValueInteger (Variables|/Game/Widgets/Select_Class_WDG.Select_Class_WDG_C|GetC_Zeon Widget) _c_zeon)
  (CallFunction|SetValueInteger (Variables|/Game/Widgets/Select_Class_WDG.Select_Class_WDG_C|GetC_ACT Widget) _c_act)
  (CallFunction|SetValueInteger (Variables|/Game/Widgets/Select_Class_WDG.Select_Class_WDG_C|GetC_ProjM Widget) _c_projmag)
  (CallFunction|SetValueInteger (Variables|/Game/Widgets/Select_Class_WDG.Select_Class_WDG_C|GetC_Conv Widget) _c_convocar)
  (CallFunction|SetValueInteger (Variables|/Game/Widgets/Select_Class_WDG.Select_Class_WDG_C|GetC_Domin Widget) _c_dominar)
  (CallFunction|SetValueInteger (Variables|/Game/Widgets/Select_Class_WDG.Select_Class_WDG_C|GetC_Atar Widget) _c_atar)
  (CallFunction|SetValueInteger (Variables|/Game/Widgets/Select_Class_WDG.Select_Class_WDG_C|GetC_Desconv Widget) _c_desconvocar)
  (CallFunction|SetValueInteger (Variables|/Game/Widgets/Select_Class_WDG.Select_Class_WDG_C|GetC_Limite_Psi Widget) _limite_psi)
  (CallFunction|SetValueInteger (Variables|/Game/Widgets/Select_Class_WDG.Select_Class_WDG_C|GetC_CV Widget) _c_cv)
  (CallFunction|SetValueInteger (Variables|/Game/Widgets/Select_Class_WDG.Select_Class_WDG_C|GetC_Proj_Psi Widget) _c_projpsi)
  (CallFunction|SetValueInteger (Variables|/Game/Widgets/Select_Class_WDG.Select_Class_WDG_C|GetC_Atleticas Widget) _c_atleticas)
  (CallFunction|SetValueInteger (Variables|/Game/Widgets/Select_Class_WDG.Select_Class_WDG_C|GetC_Sociales Widget) _c_sociales)
  (CallFunction|SetValueInteger (Variables|/Game/Widgets/Select_Class_WDG.Select_Class_WDG_C|GetC_Perceptivas Widget) _c_perceptivas)
  (CallFunction|SetValueInteger (Variables|/Game/Widgets/Select_Class_WDG.Select_Class_WDG_C|GetC_Intelectuales Widget) _c_intelectuales)
  (CallFunction|SetValueInteger (Variables|/Game/Widgets/Select_Class_WDG.Select_Class_WDG_C|GetC_Vigor Widget) _c_vigor)
  (CallFunction|SetValueInteger (Variables|/Game/Widgets/Select_Class_WDG.Select_Class_WDG_C|GetC_Subterfugio Widget) _c_subterfugio)
  (CallFunction|SetValueInteger (Variables|/Game/Widgets/Select_Class_WDG.Select_Class_WDG_C|GetC_Creativas Widget) _c_creativas)
  (CallFunction|SetValueInteger (Variables|/Game/Widgets/Select_Class_WDG.Select_Class_WDG_C|GetB_Ataque Widget) _b_lvl_ataque)
  (CallFunction|SetValueInteger (Variables|/Game/Widgets/Select_Class_WDG.Select_Class_WDG_C|GetB_Esquiva Widget) _b_lvl_esquiva)
  (CallFunction|SetValueInteger (Variables|/Game/Widgets/Select_Class_WDG.Select_Class_WDG_C|GetB_Parada Widget) _b_lvl_parada)
  (CallFunction|SetValueInteger (Variables|/Game/Widgets/Select_Class_WDG.Select_Class_WDG_C|GetB_Armadura Widget) _b_lvl_armadura)
  (CallFunction|SetValueInteger (Variables|/Game/Widgets/Select_Class_WDG.Select_Class_WDG_C|GetB_Zeon Widget) _b_zeon)
  (CallFunction|SetValueInteger (Variables|/Game/Widgets/Select_Class_WDG.Select_Class_WDG_C|GetB_Convocar Widget) _b_convocar)
  (CallFunction|SetValueInteger (Variables|/Game/Widgets/Select_Class_WDG.Select_Class_WDG_C|GetB_Dominar Widget) _b_dominar)
  (CallFunction|SetValueInteger (Variables|/Game/Widgets/Select_Class_WDG.Select_Class_WDG_C|GetB_Atar Widget) _b_atar)
  (CallFunction|SetValueInteger (Variables|/Game/Widgets/Select_Class_WDG.Select_Class_WDG_C|GetB_Desconvocar Widget) _b_desconvocar)
  (return))

(fn SetValueString
  (params (Name :type Text%20Block%20Object%20Reference) (Value :type String))
  (Rendering|Components|TextRender|SetText Name (Utilities|Text|ToText(String) Value))
  (return))

(fn SetValueInteger
  (params (Name :type Text%20Block%20Object%20Reference) (Value :type Integer))
  (Rendering|Components|TextRender|SetText Name (Utilities|Text|ToText(Integer) Value))
  (return))

(fn SetPD
  (params (Text :type Text%20Block%20Object%20Reference) (Value :type Text))
  (Rendering|Components|TextRender|SetText Text (Utilities|Text|ToText(Integer) (+ (* (Math|Conversions|ToInteger(Byte) (Utilities|String|ToString(Text) Value)) 100) 500))))

(fn AttributeChanged
  (params (Text :type Editable%20Text%20Box%20Object%20Reference) (Value :type Text))
  (switch string (Utilities|GetObjectName Text)))

(event Custom|ChangePDEvent
  (params (Text :type Text%20%28by%20ref%29) (CommitMethod :type ETextCommit%20Enum :default "Default"))
  (switch Utilities|FlowControl|Switch|SwitchonETextCommit CommitMethod
    (:Default
      _)
    (:OnEnter
      _)
    (:OnUserMovedFocus
      _)
    (:OnCleared
      _))
  (CallFunction|SetPD (Variables|/Game/Widgets/Select_Class_WDG.Select_Class_WDG_C|GetPD_Totales (stale _self2)) Text))

(event Custom|ChangeCategoryEvent
  (params (SelectedItem :type String) (SelectionType :type ESelectInfo%20Enum :default "OnKeyPress"))
  (for _array_element (Variables|/Game/Blueprints/BP_AnimaCreatorGameMode.BP_AnimaCreatorGameMode_C|GetCategoriaArray (Variables|Default|GetGameMode))
    (if (Utilities|Enum|Equal(Enum) SelectedItem (Utilities|String|ToString(Name) (.Categoria (Utilities|Struct|BreakStruct_Categoria _array_element))))
      (CallFunction|SetFields _array_element (Variables|Default|GetCategorias_WDG)))))